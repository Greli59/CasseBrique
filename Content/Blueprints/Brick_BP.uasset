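; Destructible brick actor that loses one health each time an actor tagged "Ball" hits it and destroys itself at zero.
; Health starts at MaxHealth on BeginPlay, and each non-lethal hit refreshes the brick's color.
; UpdateColor picks the BaseColor array entry matching current health and writes it to the Cube's "Tint" custom primitive data parameter.
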(event EventBeginPlay
  (Variables|Default|SetCurrentHealth (Variables|Default|GetMaxHealth))
  (CallFunction|UpdateColor))

(event Collision|EventHit
  (params (MyComp :type Primitive%20Component%20Object%20Reference) (Other :type Actor%20Object%20Reference) (OtherComp :type Primitive%20Component%20Object%20Reference) (bSelfMoved :type Boolean) (HitLocation :type Vector :default "0, 0, 0") (HitNormal :type Vector :default "0, 0, 0") (NormalImpulse :type Vector :default "0, 0, 0") (Hit :type Hit%20Result%20Structure%20%28by%20ref%29))
  (if (Actor|ActorHasTag Other "Ball")
    (bind _result (Math|Integer|DecrementInt (Variables|Default|GetCurrentHealth))
      (:%20%20
        (Variables|Default|SetCurrentHealth _result)
        (if (== (Variables|Default|GetCurrentHealth) 0)
          (Actor|DestroyActor)
          (else
            (CallFunction|UpdateColor)))))))

(fn ConstructionScript)

(fn UpdateColor
  (bind _currenthealth (Variables|Default|GetCurrentHealth))
  (bind _basecolor (Variables|Default|GetBaseColor))
  (bind _basecolor_2 (Variables|Default|GetBaseColor))
  (bind _returnvalue (Utilities|Array|Length _basecolor))
  (bind _returnvalue_2 (Math|Integer|Clamp(Integer) _currenthealth 0 _returnvalue))
  (bind _returnvalue_3 (- _returnvalue_2 1))
  (bind _output (Utilities|Array|Get(acopy) _basecolor_2 _returnvalue_3))
  (Class|PrimitiveComponent|SetVectorParameterforCustomPrimitiveData (Variables|Default|GetCube) "Tint" (Math|Vector4|MakeVector4 (.r _output) (.g _output) (.b _output) (.a _output))))
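; Ball actor for a paddle-and-ball game, driven by a physics-simulated Sphere that launches along -X at BeginPlay.
; Tick renormalizes the linear velocity to Speed, keeping the ball at constant speed through collisions.
; On hitting an actor tagged "Paddle", it redirects the ball toward +X, angled by the clamped Y offset of the impact from the paddle center, preserving velocity magnitude.
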(event OnComponentHit(Sphere)
  (params (HitComponent :type Primitive%20Component%20Object%20Reference) (OtherActor :type Actor%20Object%20Reference) (OtherComp :type Primitive%20Component%20Object%20Reference) (NormalImpulse :type Vector :default "0, 0, 0") (Hit :type Hit%20Result%20Structure%20%28by%20ref%29))
  ;[0.15 0.15 0.15 0.5] Bounce on paddle
  ;;[0.15 0.15 0.15 0.5] Check if it is a paddle
  (if (Actor|ActorHasTag OtherActor "Paddle")
    (bind _returnvalue (Physics|GetPhysicsLinearVelocity (Variables|Default|GetSphere) "None"))
    (Physics|SetPhysicsLinearVelocity (Variables|Default|GetSphere) (* (Math|Vector|VectorLength _returnvalue) (Math|Vector|Normalize (Math|Vector|MakeVector 1.0 (Math|Float|Clamp(Float) (/ (- (.y (.impactpoint Hit)) (.y (Transformation|GetActorLocation OtherActor))) 2.5e+02) -1.0) 0.0))) false "None")))

(event EventBeginPlay
  ;[0.15 0.15 0.15 0.5] Vitesse initiale
  (Physics|AddImpulse (Variables|Default|GetSphere) (Math|Vector|MakeVector (* (Variables|Default|GetSpeed) -1.0) 0.0 0.0) "None" true))

(event EventTick
  (params (DeltaSeconds :type Float%20%28single-precision%29))
  ;[0.15 0.15 0.15 0.5] Maintenir la vitesse constante
  (bind _returnvalue (Physics|GetPhysicsLinearVelocity (Variables|Default|GetSphere) "None"))
  (Physics|SetPhysicsLinearVelocity (Variables|Default|GetSphere) (* (Math|Vector|Normalize _returnvalue) (Variables|Default|GetSpeed)) false "None"))

(fn ConstructionScript)